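; Laser actor that line-traces forward every tick and bounces off reflective-material surfaces up to a bounce limit.
; LaserMath mirrors the ray about the hit actor's forward vector, and CanReflect gates bounces on material and a perpendicularity test.
; It sets or clears the hit component on BP_Prism actors and applies damage after the bounce loop.
; The EnableLaser beam-particle call is disconnected, leaving only trace debug drawing to show the path.
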(event `self.ReceiveTick`
  (params (DeltaSeconds :type "Float (single-precision)"))
  (`self.CalculateTrajectory`))

(fn `CalculateTrajectory`
  (bind _hit_actor (`self.Hit Actor`))
  (bind _raytracelimittemp (`self.RaytraceLimitTemp`))
  (bind _returnvalue (`self.K2_GetActorLocation` self))
  ;[1 1 1] First Laser
  (set `self.TempLocation` _returnvalue)
  (bind (_outhit _returnvalue_2) (`KismetSystemLibrary.LineTraceSingle` :`Start` _returnvalue :`End` (+ _returnvalue (* (`KismetMathLibrary.GetForwardVector` (`self.K2_GetActorRotation` self)) (`self.Distance`))) :`TraceChannel` "TraceTypeQuery3" :`DrawDebugType` (`self.Raytrace Debug Enum`)))
  (if _returnvalue_2
    (bind (_bblockinghit _binitialoverlap _time _location _impactpoint _normal _impactnormal _physmat _hitactor _hitcomponent) (`GameplayStatics.BreakHitResult` _outhit))
    (set `self.HitLocation` _location)
    (set `self.Hit Actor` _hitactor)
    (set `self.Hit_Component` _hitcomponent)
    (set `self.HitMaterial` (`PrimitiveComponent.GetMaterial` _hitcomponent 0))
    (bind (_isperpendicular_ _reflection) (`self.LaserMath` (`self.HitLocation`) _returnvalue (`self.Hit Actor`) self _normal))
    (set `self.EndLocation` (* _reflection (`self.Distance`)))
    (bind _canreflect_ (`self.CanReflect` _isperpendicular_ (`self.HitMaterial`)))
    (if _canreflect_
      (set `self.StartLocation` (`self.HitLocation`))
      ;[1 1 1] For every bounce
      (while (`self.Continue?`)
        (bind (_outhit_2 _returnvalue_3) (`KismetSystemLibrary.LineTraceSingle` :`Start` (`self.StartLocation`) :`End` (`self.EndLocation`) :`TraceChannel` "TraceTypeQuery3" :`DrawDebugType` (`self.Raytrace Debug Enum`)))
        (if _returnvalue_3
          (bind (_bblockinghit_2 _binitialoverlap_2 _time_2 _location_2 _impactpoint_2 _normal_2 _impactnormal_2 _physmat_2 _hitactor_2 _hitcomponent_2) (`GameplayStatics.BreakHitResult` _outhit_2))
          (set `self.HitLocation` _location_2)
          (set `self.Hit Actor` _hitactor_2)
          (set `self.Hit_Component` _hitcomponent_2)
          (set `self.HitMaterial` (`PrimitiveComponent.GetMaterial` _hitcomponent_2 0))
          (bind (_isperpendicular__2 _reflection_2) (`self.LaserMath` (`self.HitLocation`) (`self.StartLocation`) (`self.Hit Actor`) self))
          (set `self.EndLocation` (* _reflection_2 (`self.Distance`)))
          (bind _canreflect__2 (`self.CanReflect` _isperpendicular__2 (`self.HitMaterial`)))
          (if (and _canreflect__2 (not (== _raytracelimittemp (`self.RaytraceLimit`))))
            (set `self.StartLocation` (`self.HitLocation`))
            (set `self.RaytraceLimitTemp` (+ _raytracelimittemp 1)))
          (else
            (bind _asbp_prism (cast `/Game/Blueprints/BP_Prism` _hit_actor :!label _label))
            (set `/Game/Blueprints/BP_Prism.Hit_Component` (`self.Null_Object`) _asbp_prism))))
      (set `self.RaytraceLimitTemp` 0)
      (`GameplayStatics.ApplyDamage` (`self.Hit Actor`) (`self.Base_Damage`) null self)
      (else
        (if false
          _
          (else
            _))
        (bind _asbp_prism_2 (cast `/Game/Blueprints/BP_Prism` _hit_actor))
        (set `/Game/Blueprints/BP_Prism.Hit_Component` (`self.Hit_Component`) _asbp_prism_2)))
    (else
      (goto _label))))

(fn `CanReflect`
  (params (`IsPerpendicular?` :type Boolean) (`Hit Mat` :type "MaterialInterface Object Reference"))
  (returns (`CanReflect?` :type Boolean))
  (bind _returnvalue (`MaterialInterface.GetBaseMaterial` `Hit Mat`))
  (return (and (not `IsPerpendicular?`) (== _returnvalue (`self.ReflectiveMaterial`)) (not (== `Hit Mat` null)))))

(fn `EnableLaser`
  (params (StartPoint :type "Vector Structure") (EndPoint :type "Vector Structure"))
  (bind _returnvalue (`GameplayStatics.SpawnEmitterAtLocation` null StartPoint))
  (bind _output_get (set `self.P_Laser` _returnvalue))
  (`ParticleSystemComponent.SetBeamSourcePoint` _output_get 0 StartPoint 0)
  (`ParticleSystemComponent.SetBeamEndPoint` _output_get 0 EndPoint))

(fn `LaserMath`
  (params (`Hit Location` :type "Vector Structure") (Start :type "Vector Structure") (`Hit Actor` :type "Actor Object Reference") (`Self Actor` :type "Actor Object Reference") (HitNormal :type "Vector Structure"))
  (returns (`IsPerpendicular?` :type Boolean) (Reflection :type "Vector Structure"))
  (bind _returnvalue (`KismetMathLibrary.Normal` (`self.GetActorForwardVector` `Hit Actor`)))
  (bind _returnvalue_2 (`KismetMathLibrary.MakeVector` (- (.x `Hit Location`) (.x Start)) (- (.y `Hit Location`) (.y Start)) (- (.z `Hit Location`) (.z Start))))
  (return (== (`KismetMathLibrary.DegAcos` (`KismetMathLibrary.Dot_VectorVector` (`KismetMathLibrary.Normal` HitNormal) (`KismetMathLibrary.Normal` Start))) 0.0) (`KismetMathLibrary.Normal` (`KismetMathLibrary.MakeVector` (.x (- (* (* _returnvalue 2) (`KismetMathLibrary.Dot_VectorVector` _returnvalue_2 _returnvalue)) _returnvalue_2)) (+ (.y (- (* (* _returnvalue 2) (`KismetMathLibrary.Dot_VectorVector` _returnvalue_2 _returnvalue)) _returnvalue_2)) 0.0) (.z (- (* (* _returnvalue 2) (`KismetMathLibrary.Dot_VectorVector` _returnvalue_2 _returnvalue)) _returnvalue_2))))))

(fn `UserConstructionScript`)