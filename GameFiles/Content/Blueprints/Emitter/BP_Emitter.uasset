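; Emitter actor that keeps a spawned instance of SpawnClass alive while its Enabled flag is on.
; Tick compares Enabled with EnabledOld and uses a DoOnce, reset on change, to spawn once per enable; disabling destroys the spawned actor.
; The actor spawns at EmitterLocation's relative transform, then Tick snaps it to that component's world transform every frame.
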(event `self.ReceiveTick`
  (params (DeltaSeconds :type "Float (single-precision)"))
  (bind _enabled_ (`self.Enabled?`))
  (bind _spawned_actor (`self.Spawned_Actor`))
  (bind _spawned_actor_2 (`self.Spawned_Actor`))
  (`|ExecutionSequence`
    (:`then_0`
      (if (`self.Enabled?`)
        (if (not (== _enabled_ (`self.EnabledOld`)))
          (`|ExecutionSequence`
            (:`then_0`
              (goto _label :!via `Reset`))
            (:`then_1`
              _)))
        (`/Engine/EditorBlueprintResources/StandardMacros.DoOnce` false :!label _label
          (:`Completed`
            (set `self.EnabledOld` (`self.Enabled?`))
            (bind _returnvalue (`|SpawnActorFromClass` (`self.SpawnClass`) (`SceneComponent.GetRelativeTransform` (`self.Emitter_Location`)) "Undefined" "OverrideRootScale"))
            (set `self.Spawned_Actor` _returnvalue)))
        (else
          (set `self.EnabledOld` _enabled_)
          (if (!= _spawned_actor null)
            (`self.K2_DestroyActor` _spawned_actor)))))
    (:`then_1`
      (if (!= _spawned_actor_2 null)
        (`self.K2_SetActorTransform` _spawned_actor_2 (`SceneComponent.K2_GetComponentToWorld` (`self.Emitter_Location`)) false false)))))

(fn `UserConstructionScript`)