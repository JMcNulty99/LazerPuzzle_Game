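; BP_Prism is a prism actor that splits a laser hitting one of its three sides into two outgoing beams.
; Each Tick compares HitComponent, which is not set in this graph, against LastHitComponent to react only to changes.
; A newly hit side spawns BP_Laser actors at the other two sides' emitter transforms.
; Both lasers are destroyed only when HitComponent clears, so switching directly between sides leaves the previous pair alive.
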(event `self.ReceiveTick`
  (params (DeltaSeconds :type "Float (single-precision)"))
  (bind _hit_component (`self.Hit_Component`))
  (bind _lazer_side_b (`self.Lazer_Side_B`))
  (bind _lazer_side_a (`self.Lazer_Side_A`))
  (if (== _hit_component null)
    (if (not (== _lazer_side_a null))
      (`self.K2_DestroyActor` _lazer_side_a))
    (if (not (== _lazer_side_b null))
      (`self.K2_DestroyActor` _lazer_side_b))
    (set `self.Last_Hit_Component` null)
    (elif (not (== _hit_component (`self.Last_Hit_Component`)))
      (if (== _hit_component (`self.SideOne`))
        (bind _returnvalue (`|SpawnActorFromClass` "/Game/Blueprints/BP_Laser.BP_Laser_C" (`SceneComponent.K2_GetComponentToWorld` (`self.E_Side_Two`)) "Undefined" "OverrideRootScale"))
        (set `self.Lazer_Side_A` _returnvalue)
        (bind _returnvalue_2 (`|SpawnActorFromClass` "/Game/Blueprints/BP_Laser.BP_Laser_C" (`SceneComponent.K2_GetComponentToWorld` (`self.E_Side_Three`)) "Undefined" "OverrideRootScale"))
        (set `self.Lazer_Side_B` _returnvalue_2)
        (set `self.Last_Hit_Component` (`self.Hit_Component`) :!label _label)
        (elif (== _hit_component (`self.SideTwo`))
          (bind _returnvalue_3 (`|SpawnActorFromClass` "/Game/Blueprints/BP_Laser.BP_Laser_C" (`SceneComponent.K2_GetComponentToWorld` (`self.E_Side_One`)) "Undefined" "OverrideRootScale"))
          (set `self.Lazer_Side_A` _returnvalue_3)
          (bind _returnvalue_4 (`|SpawnActorFromClass` "/Game/Blueprints/BP_Laser.BP_Laser_C" (`SceneComponent.K2_GetComponentToWorld` (`self.E_Side_Three`)) "Undefined" "OverrideRootScale"))
          (set `self.Lazer_Side_B` _returnvalue_4)
          (goto _label)
          (elif (== _hit_component (`self.SideThree`))
            (bind _returnvalue_5 (`|SpawnActorFromClass` "/Game/Blueprints/BP_Laser.BP_Laser_C" (`SceneComponent.K2_GetComponentToWorld` (`self.E_Side_One`)) "Undefined" "OverrideRootScale"))
            (set `self.Lazer_Side_A` _returnvalue_5)
            (bind _returnvalue_6 (`|SpawnActorFromClass` "/Game/Blueprints/BP_Laser.BP_Laser_C" (`SceneComponent.K2_GetComponentToWorld` (`self.E_Side_Two`)) "Undefined" "OverrideRootScale"))
            (set `self.Lazer_Side_B` _returnvalue_6)
            (goto _label)))))))

(fn `UserConstructionScript`)