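; Prism actor that, when one of its three sides is hit, spawns an actor of SpawnClass at the other two, acting as a splitter.
; Tick polls HitComponent, which is not set in this graph, and uses a DoOnce per side to spawn once per hit.
; A change of hit component resets those gates and destroys the spawned actors.
; L_Activate and L_Deactivate toggle component visibility and tick but are not called here.
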(event `self.ReceiveTick`
  (params (DeltaSeconds :type "Float (single-precision)"))
  (bind _spawn_class (`self.Spawn_Class`))
  (bind _spawn_class_2 (`self.Spawn_Class`))
  (bind _side_a (`self.Side_A`))
  (bind _side_b (`self.Side_B`))
  (bind _side_c (`self.Side_C`))
  (bind _side_a_2 (`self.Side_A`))
  (bind _side_b_2 (`self.Side_B`))
  (bind _side_c_2 (`self.Side_C`))
  (if (!= (`self.Hit_Component`) (`self.Hit_Component_Old`))
    (`|ExecutionSequence`
      (:`then_0`
        (goto _label :!via `Reset`))
      (:`then_1`
        (goto _label_2 :!via `Reset`))
      (:`then_2`
        (goto _label_3 :!via `Reset`))
      (:`then_3`
        (set `self.Hit_Component_Old` (`self.Hit_Component`))
        (if (!= _side_a_2 null)
          (`self.K2_DestroyActor` _side_a_2))
        (if (!= _side_b_2 null)
          (`self.K2_DestroyActor` _side_b_2))
        (if (!= _side_c_2 null)
          (`self.K2_DestroyActor` _side_c_2))))
    (elif (== (`self.Hit_Component`) (`self.SideOne`))
      (`/Engine/EditorBlueprintResources/StandardMacros.DoOnce` true :!label _label
        (:`Completed`
          (bind _returnvalue (`|SpawnActorFromClass` _spawn_class (`SceneComponent.K2_GetComponentToWorld` (`self.Side_Two`)) "Undefined" "OverrideRootScale"))
          (set `self.Side_B` _returnvalue)
          (bind _returnvalue_2 (`|SpawnActorFromClass` _spawn_class_2 (`SceneComponent.K2_GetComponentToWorld` (`self.Side_Three`)) "Undefined" "OverrideRootScale"))
          (set `self.Side_C` _returnvalue_2)
          (if (!= _side_a null)
            (`self.K2_DestroyActor` _side_a))))
      (elif (== (`self.Hit_Component`) (`self.SideTwo`))
        (`/Engine/EditorBlueprintResources/StandardMacros.DoOnce` true :!label _label_2
          (:`Completed`
            (bind _returnvalue_3 (`|SpawnActorFromClass` _spawn_class (`SceneComponent.K2_GetComponentToWorld` (`self.Side_One`)) "Undefined" "OverrideRootScale"))
            (set `self.Side_A` _returnvalue_3)
            (bind _returnvalue_4 (`|SpawnActorFromClass` _spawn_class_2 (`SceneComponent.K2_GetComponentToWorld` (`self.Side_Three`)) "Undefined" "OverrideRootScale"))
            (set `self.Side_C` _returnvalue_4)
            (if (!= _side_b null)
              (`self.K2_DestroyActor` _side_b))))
        (elif (== (`self.Hit_Component`) (`self.SideThree`))
          (`/Engine/EditorBlueprintResources/StandardMacros.DoOnce` true :!label _label_3
            (:`Completed`
              (bind _returnvalue_5 (`|SpawnActorFromClass` _spawn_class (`SceneComponent.K2_GetComponentToWorld` (`self.Side_One`)) "Undefined" "OverrideRootScale"))
              (set `self.Side_A` _returnvalue_5)
              (bind _returnvalue_6 (`|SpawnActorFromClass` _spawn_class_2 (`SceneComponent.K2_GetComponentToWorld` (`self.Side_Two`)) "Undefined" "OverrideRootScale"))
              (set `self.Side_B` _returnvalue_6)
              (if (!= _side_c null)
                (`self.K2_DestroyActor` _side_c)))))))))

(fn `L_Activate`
  (params (Actor :type "ChildActorComponent Object Reference"))
  (`SceneComponent.SetVisibility` Actor true true)
  (`ActorComponent.SetComponentTickEnabled` Actor true)
  (return))

(fn `L_Deactivate`
  (params (Actor :type "ChildActorComponent Object Reference"))
  (`SceneComponent.SetVisibility` Actor false true)
  (`ActorComponent.SetComponentTickEnabled` Actor false)
  (return))

(fn `UserConstructionScript`)