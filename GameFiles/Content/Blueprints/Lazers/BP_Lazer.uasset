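; BP_Lazer is a laser actor that casts a bouncing beam from its forward direction every tick.
; A do-while macro repeats LazerLogic, reflecting each line trace off the hit normal until it misses, exceeds the bounce limit or fails an angle check.
; Hit BP_Prism actors receive the struck component, with logic to clear the last one; other receiver types are stubbed.
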(event `self.ReceiveTick`
  (params (DeltaSeconds :type "Float (single-precision)"))
  (set `self.StartLocation` (`self.K2_GetActorLocation` self))
  (set `self.EndLocation` (`KismetMathLibrary.GetForwardVector` (`self.K2_GetActorRotation` self)))
  (set `self.RaytraceLimitTemp` 0)
  (`self.DoWhile` (`self.CanReflect?`)
    (:`Loop Body`
      (`self.LazerLogic`))))

(fn `CanReflect`
  (params (`Start Location` :type "Vector Structure") (`Hit Normal` :type "Vector Structure"))
  (returns (`CanRelfect?` :type Boolean))
  (return (not (== (`KismetMathLibrary.DegAcos` (`KismetMathLibrary.Dot_VectorVector` (`KismetMathLibrary.Normal` `Hit Normal`) (`KismetMathLibrary.Normal` `Start Location`))) 0.0))))

(fn `DeleteParticles`
  (if (not (== (`KismetArrayLibrary.Array_Length` (`self.Emitters`)) 0))
    (for _array_element _
      (`self.K2_DestroyActor` _array_element)))
  (return))

(fn `LazerLogic`
  (bind _lasthitactor (`self.LastHitActor`))
  (bind _startlocation (`self.StartLocation`))
  (bind _raytracelimittemp (`self.RaytraceLimitTemp`))
  (bind (_outhit _returnvalue) (`KismetSystemLibrary.LineTraceSingle` :`Start` _startlocation :`End` (+ _startlocation (* (`self.EndLocation`) (`self.Distance`))) :`TraceChannel` "TraceTypeQuery3" :`DrawDebugType` (`self.Raytrace Debug Enum`) :`DrawTime` 0.5))
  (if _returnvalue
    (bind (_bblockinghit _binitialoverlap _time _location _impactpoint _normal _impactnormal _physmat _hitactor _hitcomponent _hitbonename _hititem _faceindex _tracestart) (`GameplayStatics.BreakHitResult` _outhit))
    (set `self.EndLocation` (`KismetMathLibrary.GetReflectionVector` (`KismetMathLibrary.Normal` (- _location _tracestart)) (`KismetMathLibrary.Normal` _impactnormal)))
    (set `self.StartLocation` _location)
    (set `self.CanReflect?` (and (`self.CanReflect` _tracestart _impactnormal) (<= _raytracelimittemp (`self.RaytraceLimit`))))
    (`/Engine/EditorBlueprintResources/StandardMacros.IncrementInt` _raytracelimittemp
      (:`  `
        (if (!= _hitactor null)
          (bind _asbp_prism (cast `/Game/Blueprints/Prisms/BP_Prism` _hitactor)
            (:`then`
              (set `/Game/Blueprints/Prisms/BP_Prism.Hit_Component` _hitcomponent _asbp_prism))
            (:`CastFailed`
              (if true
                _
                (else
                  _))))
          (set `self.LastHitActor` _hitactor) ; set LAST
          (elif (!= _lasthitactor null)
            (bind _asbp_prism_2 (cast `/Game/Blueprints/Prisms/BP_Prism` _lasthitactor)
              (:`then`
                (set `/Game/Blueprints/Prisms/BP_Prism.Hit_Component` null _asbp_prism_2))
              (:`CastFailed`
                (if true
                  _
                  (else
                    _))))
            (set `self.LastHitActor` null) ; set last
          ))))
    (else
      (set `self.CanReflect?` false))))

(fn `UserConstructionScript`)