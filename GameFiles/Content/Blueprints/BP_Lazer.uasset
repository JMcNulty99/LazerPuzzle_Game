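; BP_Lazer is a laser actor that fires a bouncing line trace from its forward vector every tick.
; A custom DoWhile macro repeats LazerLogic, which reflects the direction off each impact normal and restarts from the hit point.
; Bouncing stops on a miss, at RaytraceLimit, or when CanReflect finds the normalized trace start position aligned with the hit normal.
; The only visual is the trace's debug draw.
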(event `self.ReceiveTick`
  (params (DeltaSeconds :type "Float (single-precision)"))
  (set `self.StartLocation` (`self.K2_GetActorLocation` self))
  (set `self.EndLocation` (`KismetMathLibrary.GetForwardVector` (`self.K2_GetActorRotation` self)))
  (set `self.RaytraceLimitTemp` 0)
  (`self.DoWhile` (`self.CanReflect?`)
    (:`Loop Body`
      (`self.LazerLogic`))))

(fn `CanReflect`
  (params (`Start Location` :type "Vector Structure") (`Hit Normal` :type "Vector Structure"))
  (returns (`CanRelfect?` :type Boolean))
  (return (not (== (`KismetMathLibrary.DegAcos` (`KismetMathLibrary.Dot_VectorVector` (`KismetMathLibrary.Normal` `Hit Normal`) (`KismetMathLibrary.Normal` `Start Location`))) 0.0))))

(fn `LazerLogic`
  (bind _startlocation (`self.StartLocation`))
  (bind _raytracelimittemp (`self.RaytraceLimitTemp`))
  (bind (_outhit _returnvalue) (`KismetSystemLibrary.LineTraceSingle` :`Start` _startlocation :`End` (+ _startlocation (* (`self.EndLocation`) (`self.Distance`))) :`TraceChannel` "TraceTypeQuery3" :`DrawDebugType` (`self.Raytrace Debug Enum`) :`TraceHitColor` (struct) :`DrawTime` 0.05))
  (if _returnvalue
    (bind (_bblockinghit _binitialoverlap _time _location _impactpoint _normal _impactnormal _physmat _hitactor _hitcomponent _hitbonename _hititem _faceindex _tracestart) (`GameplayStatics.BreakHitResult` _outhit))
    (set `self.EndLocation` (`KismetMathLibrary.GetReflectionVector` (`KismetMathLibrary.Normal` (- _location _tracestart)) (`KismetMathLibrary.Normal` _impactnormal)))
    (set `self.StartLocation` _location)
    (set `self.CanReflect?` (and (`self.CanReflect` _tracestart _impactnormal) (<= _raytracelimittemp (`self.RaytraceLimit`))))
    (`/Engine/EditorBlueprintResources/StandardMacros.IncrementInt` _raytracelimittemp)
    (else
      (set `self.CanReflect?` false))))

(fn `UserConstructionScript`)